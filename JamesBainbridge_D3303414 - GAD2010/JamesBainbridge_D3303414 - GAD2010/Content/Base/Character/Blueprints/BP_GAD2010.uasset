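; Player character Blueprint with camera-relative movement, short and hold-to-progress interactions, and a banish-style death.
; An InteractorController drives material highlighting and interaction attempts, which feed a montage or a progress widget.
; A gate blocks long interactions from repeating until input is released.
; Any damage raises and flares the mesh, fades the screen, then requests an EncounterGameMode respawn or reopens the level without that mode.
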(event Input|EnhancedActionEvents|EnhancedInputActionIA_Move
  (params (ActionValue :type Vector%202D%20Structure) (ElapsedSeconds :type Float%20%28double-precision%29) (TriggeredSeconds :type Float%20%28double-precision%29) (InputAction :type Input%20Action%20Object%20Reference :default "/Game/Base/Input/IA_Move.IA_Move"))
  (|Movement ActionValue))

(event Input|EnhancedActionEvents|EnhancedInputActionIA_BasicInteraction
  (params (ActionValue :type Boolean) (ElapsedSeconds :type Float%20%28double-precision%29) (TriggeredSeconds :type Float%20%28double-precision%29) (InputAction :type Input%20Action%20Object%20Reference :default "/Game/Base/Input/IA_BasicInteraction.IA_BasicInteraction"))
  (if (CallFunction|CanInteract)
    (|ShortInteraction)))

(event Input|EnhancedActionEvents|EnhancedInputActionIA_LongInteraction
  (params (ActionValue :type Boolean) (ElapsedSeconds :type Float%20%28double-precision%29) (TriggeredSeconds :type Float%20%28double-precision%29) (InputAction :type Input%20Action%20Object%20Reference :default "/Game/Base/Input/IA_LongInteraction.IA_LongInteraction"))
  (:Triggered
    (if (CallFunction|CanInteract)
      (|LongInteraction :!label _label)))
  (:Completed
    (goto _label Completed)))

(event EventBeginPlay
  (|InputMapping)
  (|UI)
  (|StartingValues)
  (|EffectBindings))

(event Game|Damage|EventAnyDamage
  (params (Damage :type Float%20%28single-precision%29) (DamageType :type Damage%20Type%20Object%20Reference) (InstigatedBy :type Controller%20Object%20Reference) (DamageCauser :type Actor%20Object%20Reference))
  (|Die/Banish))

(event Input|ActionEvents|InputActionQuit
  (params (Key :type Key%20Structure :default "None"))
  (:Pressed
    (Game|QuitGame 0 "Quit" false)))

(fn ConstructionScript)

(fn CanInteract
  ;[1 1 1] Can expand to prevent rapid-fire interactions, moving interaction, etc.
  (return (Math|Boolean|NORBoolean (AI|Components|NavMovement|IsFalling (Variables|Character|GetCharacterMovement)) (Variables|Default|GetDead))))

(fn ResetValues
  (bind _bodymaterial (Variables|Default|GetBodyMaterial))
  (Transformation|SetRelativeLocation (Variables|Character|GetMesh) (Math|Vector|MakeVector 0.0 0.0 (Variables|Default|GetMeshStartZ)) false false)
  (Variables|Default|SetDead false)
  (Pawn|Components|CharacterMovement|SetMovementMode (Variables|Character|GetCharacterMovement) "MOVE_Walking" 0)
  (Rendering|Material|SetScalarParameterValue _bodymaterial "FlarePower" 0.0 :!class /Script/Engine.MaterialInstanceDynamic)
  (Rendering|Material|SetScalarParameterValue _bodymaterial "ActivePower" 0.0 :!class /Script/Engine.MaterialInstanceDynamic)
  (Utilities|FadeScreen 1.0 true))

(fn IsDead
  (return (Variables|Default|GetDead)))

(fn ActivateHighlight
  (params (Interaction%20Actor :type Actor%20Object%20Reference) (Interaction%20Component :type Interaction%20Component%20Object%20Reference))
  (if (Default|IsEnabled Interaction%20Component)
    (Rendering|Material|SetScalarParameterValue (Variables|Default|GetBodyMaterial) "ActivePower" 1.0 :!class /Script/Engine.MaterialInstanceDynamic)))

(fn DeactivateHighlight
  (params (Interaction%20Actor :type Actor%20Object%20Reference) (Interaction%20Component :type Interaction%20Component%20Object%20Reference))
  (if (< (Utilities|Array|Length (Default|GetEnabledInteractions (Variables|Default|GetInteractorController))) 1)
    (Rendering|Material|SetScalarParameterValue (Variables|Default|GetBodyMaterial) "ActivePower" 0.0 :!class /Script/Engine.MaterialInstanceDynamic)
    (Utilities|StopLongInteraction)))