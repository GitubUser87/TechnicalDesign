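; Throwable item actor that the player picks up and throws through short interactions on its InteractionComponent.
; Picking up disables physics and collision, attaches the item to the player's head socket, moves it above the player and halves its scale.
; Throwing detaches it, restores physics, collision and scale, and applies a forward impulse scaled by Speed.
; When its PickUp component overlaps an actor implementing Interact, it sends InteractMessage and destroys itself.
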(event OnShortInteraction(InteractionComponent)
  (params (Instigator :type Actor%20Object%20Reference))
  (bind _returnvalue (Game|GetPlayerCharacter 0))
  ;[0.4271 0.04004 0.04004] Interaction
  (if (Variables|Default|GetBeingCarried?)
    ;[0.003922 0 1] Throw actor
    (Transformation|DetachFromActor "KeepWorld" "KeepRelative" "KeepRelative")
    (Physics|SetSimulatePhysics (Variables|Default|GetRoot) true)
    (Collision|SetCollisionEnabled (Variables|Default|GetRoot) "QueryAndPhysics")
    (Physics|AddImpulse (Variables|Default|GetRoot) (* (Transformation|GetActorForwardVector (Game|GetPlayerCharacter 0)) (Variables|Default|GetSpeed)) "None" false)
    (Variables|Default|SetBeingCarried? false)
    (Transformation|SetActorScale3D "1.000000,1.000000,1.000000")
    (else
      ;[0.003922 0 1] Pick up actor
      (Physics|SetSimulatePhysics (Variables|Default|GetRoot) false)
      (Collision|SetCollisionEnabled (Variables|Default|GetRoot) "NoCollision")
      (Transformation|AttachActorToActor _returnvalue "head" "SnapToTarget" "KeepRelative" "KeepRelative" true)
      (Transformation|SetActorLocationAndRotation (+ (Transformation|GetActorLocation _returnvalue) (* (Transformation|GetActorForwardVector _returnvalue) "") "0.000000,0.000000,150.000000") "0, 0, 0")
      (Variables|Default|SetBeingCarried? true)
      (Transformation|SetActorScale3D "0.500000,0.500000,0.500000"))))

(event OnComponentBeginOverlap(PickUp)
  (params (OverlappedComponent :type Primitive%20Component%20Object%20Reference) (OtherActor :type Actor%20Object%20Reference) (OtherComp :type Primitive%20Component%20Object%20Reference) (OtherBodyIndex :type Integer) (bFromSweep :type Boolean) (SweepResult :type Hit%20Result%20Structure%20%28by%20ref%29))
  ;[1 0 0] Impact
  (if (Utilities|DoesObjectImplementInterface OtherActor "/Game/Added_Content/Blueprints/Interfaces/Interact.Interact_C")
    (Class|Interact|Interact(Message) OtherActor)
    (Actor|DestroyActor)))

(fn ConstructionScript)