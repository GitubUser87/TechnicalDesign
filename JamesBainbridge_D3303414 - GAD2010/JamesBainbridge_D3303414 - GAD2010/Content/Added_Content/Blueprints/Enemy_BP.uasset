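; Enemy_BP is a boss enemy that is defeated through repeated interactions over escalating phases.
; Each Interact advances it to Phase 2, then to Phase 3 with a flicker material on its cube, and finally kills it.
; Death destroys the actor and calls the OnBossDeath dispatcher.
; Its Move event wanders to random reachable nearby points, repeating only after each successful move.
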(event Custom|Move
  (AI|AIMoveTo 0 (.RandomLocation (AI|Navigation|GetRandomReachablePointinRadius (Transformation|GetActorLocation) 2.5e+03 0 0)) 0 5.0 false
    (:OnSuccess
      (CallFunction|Move))))

(event Custom|Kill
  ;[1 0 0] Kill
  (Actor|DestroyActor)
  (Development|PrintString "Hooray!")
  (Default|CallOnBossDeath))

(event Custom|Phase%202
  ;[0 1 0.0242] Phase 2
  (Development|PrintString "Phase 2 has begun")
  (Variables|Default|SetPhase2? true))

(event Custom|Phase%203
  ;[0.926 0 1] Phase 3
  (Development|PrintString "Phase 3 has begun")
  (Variables|Default|SetPhase3? true)
  (Rendering|Material|SetMaterial (Variables|Default|GetCube) 0 "/Game/Added_Content/Materials/Flicker_M.Flicker_M"))

(event EventInteract
  ;[0.3438 0 0] Phase Tree
  (if (Variables|Default|GetPhase3?)
    (CallFunction|Kill)
    (elif (Variables|Default|GetPhase2?)
      (CallFunction|Phase3)
      (else
        (CallFunction|Phase2)))))

(fn ConstructionScript)