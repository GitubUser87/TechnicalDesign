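; Boss actor that roams to random navmesh points while a looping timer fires fire rain and fireballs, throttled by Delay nodes.
; After a set time it tires, teleports to a rest point, then returns to fight.
; Each Interact advances phases, changing timings and enabling barriers, until the final one kills it and calls OnBossDeath.
; Its KillBox damages the player and clears phase flags, barriers and material, but not timings.
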(event OnComponentBeginOverlap(KillBox)
  (params (OverlappedComponent :type Primitive%20Component%20Object%20Reference) (OtherActor :type Actor%20Object%20Reference) (OtherComp :type Primitive%20Component%20Object%20Reference) (OtherBodyIndex :type Integer) (bFromSweep :type Boolean) (SweepResult :type Hit%20Result%20Structure%20%28by%20ref%29))
  (bind _returnvalue (Game|Player|GetPlayerPawn 0))
  ;[0 0.8865 1] Kill Box
  (if (== OtherActor _returnvalue)
    (Game|Damage|ApplyDamage _returnvalue 1.0 0 0)
    (Audio|PlaySound2D "/Engine/EditorSounds/Notifications/CompileFailed.CompileFailed" 1.0 1.0 0.0 0 0)
    (Variables|Default|SetPhase%202? false)
    (Variables|Default|SetPhase%203? false)
    (CallFunction|BarriersOff)
    ;[1 0.4466 0.183] Reset material
    (Rendering|Material|SetMaterial (Variables|Default|GetBoss) 0 "/Game/Base/Character/Materials/M_Alpha_Body.M_Alpha_Body")))

(event Custom|Move
  ;[0.9031 1 0] Movement
  (AI|AIMoveTo self (.RandomLocation (AI|Navigation|GetRandomReachablePointinRadius (Transformation|GetActorLocation) 2.5e+03 0 0)) 0 5.0 false
    (:OnSuccess
      (CallFunction|Move))))

(event Custom|RestPoint
  ;[1 0.8102 0.4664] Take a rest
  (if (not (Variables|Default|GetAt%20restpoint?))
    (AI|Navigation|StopMovement (Pawn|GetController))
    (Transformation|SetActorLocation (Variables|Default|GetRest) false true)
    (Variables|Default|SetAt%20restpoint? true)
    (Utilities|FlowControl|Delay (Variables|Default|GetResting))
    (Variables|Default|SetTired? false)
    (Transformation|SetActorLocation (Variables|Default|GetFight) false true)
    (Variables|Default|SetAt%20restpoint? false)
    (CallFunction|Move)))

(event Custom|Fireball
  ;[1 0.2031 0] Fireball attack
  (if (not (Variables|Default|GetTired?))
    (Utilities|FlowControl|Delay (Variables|Default|GetDelayBetweenAttack2))
    (bind _returnvalue (Game|SpawnActorfromClass "/Game/Added_Content/Blueprints/Boss/Fireball_BP.Fireball_BP_C" (Math|Transform|MakeTransform (+ (Transformation|GetActorLocation) "175.000000,0.000000,30.000000") "0, 0, 0" "1.000000,1.000000,1.000000") "Undefined" "MultiplyWithRoot" 0 0))
    (Physics|AddImpulse (Variables|/Game/Added_Content/Blueprints/Boss/Fireball_BP.Fireball_BP_C|GetSphere _returnvalue) (* "" (Variables|Default|GetSpeed)) "None" false)))

(event Custom|Fire%20Rain
  (bind _returnvalue (Transformation|GetActorLocation))
  (bind _returnvalue_2 (+ _returnvalue "0.000000,0.000000,-75.000000"))
  ;[0.2396 0.0312 0.0312] Fire Rain
  (if (Variables|Default|GetTired?)
    ;[0.9031 1 0] Movement
    (CallFunction|RestPoint)
    (else
      (Utilities|FlowControl|Sequence
        (:then_0
          (Utilities|FlowControl|Delay (Variables|Default|GetDelayBetweenAttack))
          (if (not (Variables|Default|GetAt%20restpoint?))
            (Game|SpawnActorfromClass "/Game/Added_Content/Blueprints/Boss/FireRain_BP.FireRain_BP_C" (Math|Transform|MakeTransform (Math|Vector|MakeVector (.x _returnvalue_2) 3.26e+03 (.z _returnvalue_2)) (Math|Rotator|MakeRotator 0.0 0.0 (Math|Random|RandomFloatinRange -1e+01 1e+01)) "1.000000,1.000000,1.000000") "Undefined" "MultiplyWithRoot" 0 0)))
        (:then_1
          ;[0.3704 0 0.4479] Sleepy Time
          (if (not (Variables|Default|GetDebugMode?))
            (Utilities|FlowControl|Delay (Variables|Default|GetSleepyTime))
            (Variables|Default|SetTired? true)))))))

(event Custom|Barriers%20Off
  (bind _actor_reference_2 (Variables|Default|GetActor%20Reference%202))
  ;[1 0.2723 0.5589] Turn Barriers Off
  (Rendering|SetVisibility (Variables|/Script/Engine.Actor|GetRootComponent _actor_reference_2) false true)
  (Default|DeactivateCollision _actor_reference_2))

(event Custom|Attack%20Pattern
  ;[1 1 1] Trigger attacks!
  (Utilities|Time|SetTimerbyEvent (delegate Custom|Attack) 0.5 true))

(event Custom|Attack
  ;[1 1 1] Trigger attacks!
  (if (not (Variables|Default|GetDebugMode?))
    (Utilities|FlowControl|Sequence
      (:then_0
        (CallFunction|FireRain))
      (:then_1
        (CallFunction|Fireball)))))

(event EventBeginPlay
  ;[0.9031 1 0] Movement
  (CallFunction|BarriersOff)
  (if (Variables|Default|GetDebugMode?)
    (Development|PrintString "Debug Mode Active")
    (elif (Variables|Default|GetTired?)
      (CallFunction|RestPoint)
      (else
        (CallFunction|Move)
        (CallFunction|AttackPattern)))))

(event EventInteract
  ;[0 0.01539 0.3438] Phase Tree
  (if (Variables|Default|GetPhase%203?)
    (CallFunction|KillBoss)
    (elif (Variables|Default|GetPhase%202?)
      (CallFunction|Phase3Plan)
      (else
        (CallFunction|Phase2Plan)))))

(fn ConstructionScript)

(fn Phase2Plan
  (bind _actor_reference_1 (Variables|Default|GetActor%20Reference%201))
  (Development|PrintString "Phase 2 has begun")
  (Variables|Default|SetDelayBetweenAttack 1e+01)
  (Variables|Default|SetDelayBetweenAttack2 3.0)
  (Variables|Default|SetSleepyTime 1e+01)
  (Variables|Default|SetPhase%202? true)
  (Rendering|SetVisibility (Variables|/Script/Engine.Actor|GetRootComponent _actor_reference_1) true true)
  (Default|ActivateCollision _actor_reference_1))

(fn Phase3Plan
  (bind _actor_reference_2 (Variables|Default|GetActor%20Reference%202))
  (Development|PrintString "Phase 3 has begun")
  (Variables|Default|SetPhase%203? true)
  (Rendering|Material|SetMaterial (Variables|Default|GetBoss) 0 "/Game/Added_Content/Materials/Flicker_M.Flicker_M")
  (Variables|Default|SetDelayBetweenAttack 5.0)
  (Variables|Default|SetDelayBetweenAttack2 1.5)
  (Variables|Default|SetSleepyTime 15.0)
  (Variables|Default|SetResting 3.0)
  (Rendering|SetVisibility (Variables|/Script/Engine.Actor|GetRootComponent _actor_reference_2) true true)
  (Default|ActivateCollision _actor_reference_2))

(fn KillBoss
  (Actor|DestroyActor)
  (Development|PrintString "Hooray!")
  (Default|CallOnBossDeath))

(fn GetTarget
  (return (Variables|Default|GetBoss)))