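; Short-lived boss fire rain actor that spawns fireballs repeatedly, then destroys itself four seconds after BeginPlay.
; Tick runs a sequence of five spawn branches: one every frame, the others behind staggered sub-second Delays that act as repeating timers.
; Only the three slowest branches specify Fireball_BP; the first two spawn nodes show no class.
; No spawn transform is set, and a random float node sits unused.
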(event EventTick
  (params (DeltaSeconds :type Float%20%28single-precision%29))
  ;[1 0.2457 0] Spawn Fireball/Throwable
  (Utilities|FlowControl|Sequence
    (:then_0
      (Game|SpawnActorfromClass "/Game/Added_Content/Blueprints/Boss/Fireball_BP.Fireball_BP_C" (Math|Transform|MakeTransform "0, 0, 0" "0, 0, 0" "1.000000,1.000000,1.000000") "Undefined" "MultiplyWithRoot" 0 0))
    (:then_1
      (Utilities|FlowControl|Delay 0.2)
      (Game|SpawnActorfromClass "/Game/Added_Content/Blueprints/Boss/Fireball_BP.Fireball_BP_C" (Math|Transform|MakeTransform "0, 0, 0" "0, 0, 0" "1.000000,1.000000,1.000000") "Undefined" "MultiplyWithRoot" 0 0))
    (:then_2
      (Utilities|FlowControl|Delay 0.4)
      (Game|SpawnActorfromClass "/Game/Added_Content/Blueprints/Boss/Fireball_BP.Fireball_BP_C" (Math|Transform|MakeTransform "0, 0, 0" "0, 0, 0" "1.000000,1.000000,1.000000") "Undefined" "MultiplyWithRoot" 0 0))
    (:then_3
      (Utilities|FlowControl|Delay 0.6)
      (Game|SpawnActorfromClass "/Game/Added_Content/Blueprints/Boss/Fireball_BP.Fireball_BP_C" (Math|Transform|MakeTransform "0, 0, 0" "0, 0, 0" "1.000000,1.000000,1.000000") "Undefined" "MultiplyWithRoot" 0 0))
    (:then_4
      (Utilities|FlowControl|Delay 0.8)
      (Game|SpawnActorfromClass "/Game/Added_Content/Blueprints/Boss/Fireball_BP.Fireball_BP_C" (Math|Transform|MakeTransform "0, 0, 0" "0, 0, 0" "1.000000,1.000000,1.000000") "Undefined" "MultiplyWithRoot" 0 0))))

(event EventBeginPlay
  ;[1 0 0] Self destruct
  (Utilities|FlowControl|Delay 4.0)
  (Actor|DestroyActor))

(fn ConstructionScript)