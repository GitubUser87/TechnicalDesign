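; A breakable wall actor that can be highlighted with a timed overlay material and broken through Interact, which plays a laser pull sound.
; Non-movable walls are destroyed outright, while movable ones slide along a timeline, hide when broken and respawn after a delay.
; Movable boss-defence walls start with the mesh invisible and box collision off; Activate re-enables only that collision.
; GetTarget exposes the wall mesh.
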(event Custom|Respawn
  ;[0 0.2794 1] Respawn (Only if Movable? = true)
  (if (Variables|Default|GetDestroyed)
    (Utilities|FlowControl|Delay 2e+01)
    (Rendering|SetActorHiddenInGame false)
    (Collision|SetCollisionEnabled (Variables|Default|GetWall) "QueryAndPhysics")
    (Variables|Default|SetDestroyed false)))

(event Custom|Activate
  ;[0.8893 0 1] Set collision = true
  (Collision|SetCollisionEnabled (Variables|Default|GetBox) "QueryAndPhysics"))

(event EventBeginPlay
  ;[0.278 1 0.4726] Moving?
  (if (Variables|Default|GetMovable?)
    (if (Variables|Default|GetBossDefence?)
      (Rendering|SetVisibility (Variables|Default|GetWall) false false)
      (Collision|SetCollisionEnabled (Variables|Default|GetBox) "NoCollision")
      (bind _moving (Timeline|Moving Play)
        (:Update
          (Transformation|SetRelativeLocation (Variables|Default|GetWall) _moving false false)))
      (else
        (Timeline|Moving PlayFromStart)))))

(event EventHighlight
  ;[1 1 1] Highlight
  (Rendering|Material|SetOverlayMaterial (Variables|Default|GetWall) "/Throwable_Item/Highlight_M.Highlight_M" :!class /Script/Engine.MeshComponent)
  (Utilities|FlowControl|Delay 2.0)
  (Rendering|Material|SetOverlayMaterial (Variables|Default|GetWall) 0 :!class /Script/Engine.MeshComponent))

(event EventInteract
  ;[1 0 0] Break Wall
  (Audio|PlaySound2D "/Engine/VREditor/Sounds/UI/Laser_Pull.Laser_Pull" 1.0 1.0 0.0 0 0)
  (if (Variables|Default|GetMovable?)
    (Rendering|SetActorHiddenInGame true)
    (Collision|SetCollisionEnabled (Variables|Default|GetWall) "NoCollision")
    (Variables|Default|SetDestroyed true)
    (CallFunction|Respawn)
    (else
      (Actor|DestroyActor))))

(fn ConstructionScript)

(fn GetTarget
  (return (Variables|Default|GetWall)))