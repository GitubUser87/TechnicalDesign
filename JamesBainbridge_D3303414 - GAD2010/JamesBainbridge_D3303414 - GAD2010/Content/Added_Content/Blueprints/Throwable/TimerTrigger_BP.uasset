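; A timed trigger that, when interacted with, activates a linked actor and then disappears until its timer runs out.
; Interact sends an Activate interface message to ActorReference, printing an error if that interface is missing, then hides Target and disables its collision.
; Reset restores Target's visibility and collision after TimeAvailable, without messaging the linked actor again.
; Highlight briefly applies an overlay material to Target, which GetTarget exposes.
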(event Custom|Reset
  (bind _target (Variables|Default|GetTarget))
  ;[0 0.2039 1] Reset
  (Utilities|FlowControl|Delay (Variables|Default|GetTimeAvailable))
  (Rendering|SetVisibility _target true false)
  (Collision|SetCollisionEnabled _target "QueryAndPhysics"))

(event EventHighlight
  ;[1 1 1] Highlight
  (Rendering|Material|SetOverlayMaterial (Variables|Default|GetTarget) "/Throwable_Item/Highlight_M.Highlight_M" :!class /Script/Engine.MeshComponent)
  (Utilities|FlowControl|Delay 2.0)
  (Rendering|Material|SetOverlayMaterial (Variables|Default|GetTarget) 0 :!class /Script/Engine.MeshComponent))

(event EventInteract
  (bind _actorreference (Variables|Default|GetActorReference))
  (bind _target (Variables|Default|GetTarget))
  ;[0 1 0.1326] Function
  (if (Utilities|DoesObjectImplementInterface _actorreference "/Game/Added_Content/Blueprints/Interfaces/Activate.Activate_C")
    (Class|Activate|Activate(Message) _actorreference)
    (Rendering|SetVisibility _target false false)
    (Collision|SetCollisionEnabled _target "NoCollision")
    (CallFunction|Reset)
    (else
      ;;[1 0 0] Error message if not connected
      (Development|PrintString "Not connected"))))

(fn ConstructionScript)

(fn GetTarget
  (return (Variables|Default|GetTarget)))