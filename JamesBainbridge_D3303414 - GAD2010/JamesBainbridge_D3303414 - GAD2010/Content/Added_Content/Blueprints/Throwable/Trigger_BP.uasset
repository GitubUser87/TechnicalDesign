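; Interactable trigger target that activates a linked actor through the Activate interface, then destroys itself and plays a sound.
; If the linked actor does not implement the interface, it prints a "Not connected" error instead.
; When Movable is set, a timeline started on BeginPlay drives the Target's relative location.
; A Highlight event briefly applies an overlay material to the Target, which GetTarget exposes.
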(event EventBeginPlay
  ;[0.278 1 0.4726] Moving?
  (if (Variables|Default|GetMovable?)
    (bind _moving_track (Timeline|Moving PlayFromStart)
      (:Update
        (Transformation|SetRelativeLocation (Variables|Default|GetTarget) _moving_track false false)))))

(event EventInteract
  (bind _actorreference (Variables|Default|GetActorReference))
  ;[0.01227 0 1] Main Function
  (if (Utilities|DoesObjectImplementInterface _actorreference "/Game/Added_Content/Blueprints/Interfaces/Activate.Activate_C")
    (Class|Activate|Activate(Message) _actorreference)
    (Actor|DestroyActor)
    (Audio|PlaySound2D "/Engine/VREditor/Sounds/UI/Laser_Pull.Laser_Pull" 1.0 1.0 0.0 0 0)
    (else
      ;;[1 0 0] Error message if not connected.
      (Development|PrintString "Not connected"))))

(event EventHighlight
  ;[1 1 1] Highlight
  (Rendering|Material|SetOverlayMaterial (Variables|Default|GetTarget) "/Throwable_Item/Highlight_M.Highlight_M" :!class /Script/Engine.MeshComponent)
  (Utilities|FlowControl|Delay 2.0)
  (Rendering|Material|SetOverlayMaterial (Variables|Default|GetTarget) 0 :!class /Script/Engine.MeshComponent))

(fn ConstructionScript)

(fn GetTarget
  (return (Variables|Default|GetTarget)))