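; Throwable pickup actor that the player carries overhead, then drops or throws at interactable targets.
; Interact toggles between attaching it, shrunk with physics off, and launching it by impulse.
; TargetTracker overlaps pick and highlight an Interact-implementing target; ThrowDirection aims at it when locked, otherwise along player forward.
; Hitting an interactable triggers it and destroys the item, which also self-destructs if not carried ten seconds after spawning.
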(event OnComponentBeginOverlap(TargetTracker)
  (params (OverlappedComponent :type Primitive%20Component%20Object%20Reference) (OtherActor :type Actor%20Object%20Reference) (OtherComp :type Primitive%20Component%20Object%20Reference) (OtherBodyIndex :type Integer) (bFromSweep :type Boolean) (SweepResult :type Hit%20Result%20Structure%20%28by%20ref%29))
  ;[1 0.7189 0.6079] Target Tracker
  (if (Utilities|DoesObjectImplementInterface OtherActor "/Game/Added_Content/Blueprints/Interfaces/Interact.Interact_C")
    (bind _output_get (Variables|Default|SetActorTarget OtherActor))
    (Class|Interact|Highlight(Message) _output_get)))

(event OnComponentBeginOverlap(Hit)
  (params (OverlappedComponent :type Primitive%20Component%20Object%20Reference) (OtherActor :type Actor%20Object%20Reference) (OtherComp :type Primitive%20Component%20Object%20Reference) (OtherBodyIndex :type Integer) (bFromSweep :type Boolean) (SweepResult :type Hit%20Result%20Structure%20%28by%20ref%29))
  ;[1 0 0] Impact
  (if (Utilities|DoesObjectImplementInterface OtherActor "/Game/Added_Content/Blueprints/Interfaces/Interact.Interact_C")
    (Class|Interact|Interact(Message) OtherActor)
    (Audio|PlaySound2D "/Engine/EditorSounds/Notifications/CompileSuccess.CompileSuccess" 1.0 1.0 0.0 0 0)
    (Actor|DestroyActor)))

(event OnComponentEndOverlap(TargetTracker)
  (params (OverlappedComponent :type Primitive%20Component%20Object%20Reference) (OtherActor :type Actor%20Object%20Reference) (OtherComp :type Primitive%20Component%20Object%20Reference) (OtherBodyIndex :type Integer))
  ;[1 0.7189 0.6079] Target Tracker
  (if (== OtherActor (Variables|Default|GetActorTarget))
    (bind _output_get (Variables|Default|SetActorTarget 0))
    (Class|Interact|Highlight(Message) _output_get)))

(event Custom|Interact
  (params (TargetLock :type Boolean))
  (bind _returnvalue (Game|GetPlayerCharacter 0))
  ;[0.4271 0.308 0] Interaction (Usable with any interaction system)
  (if (Variables|Default|GetBeingCarried?)
    ;[0 1 0.22] Throw actor
    (Transformation|DetachFromActor "KeepWorld" "KeepRelative" "KeepRelative")
    (Physics|SetSimulatePhysics (Variables|Default|GetThrowable) true)
    (Collision|SetCollisionEnabled (Variables|Default|GetThrowable) "QueryAndPhysics")
    (Physics|AddImpulse (Variables|Default|GetThrowable) (CallFunction|ThrowDirection TargetLock) "None" false)
    (Variables|Default|SetBeingCarried? false)
    (Transformation|SetActorScale3D "1.000000,1.000000,1.000000")
    (else
      ;[0.003922 0 1] Pick up actor
      (Physics|SetSimulatePhysics (Variables|Default|GetThrowable) false)
      (Collision|SetCollisionEnabled (Variables|Default|GetThrowable) "NoCollision")
      (Transformation|AttachActorToActor _returnvalue "head" "SnapToTarget" "KeepRelative" "KeepRelative" true)
      (Transformation|SetActorLocationAndRotation (+ (Transformation|GetActorLocation _returnvalue) (* (Transformation|GetActorForwardVector _returnvalue) "") "0.000000,0.000000,150.000000") "0, 0, 0")
      (Variables|Default|SetBeingCarried? true)
      (Transformation|SetActorScale3D "0.500000,0.500000,0.500000"))))

(event Custom|Delete
  ;[0 1 0.1781] Delete
  (Utilities|FlowControl|Delay 1e+01)
  (if (not (Variables|Default|GetBeingCarried?))
    (Actor|DestroyActor)))

(event Custom|Drop
  ;[0.647 0.3736 1] Drop function
  (Transformation|DetachFromActor "KeepWorld" "KeepRelative" "KeepRelative")
  (Physics|SetSimulatePhysics (Variables|Default|GetThrowable) true)
  (Collision|SetCollisionEnabled (Variables|Default|GetThrowable) "QueryAndPhysics")
  (Variables|Default|SetBeingCarried? false)
  (Transformation|SetActorScale3D "1.000000,1.000000,1.000000"))

(event Custom|Scan%20for%20target
  ;[1 0 0.647] Scan for target
  (Variables|Default|GetActorTarget
    (:then
      (Variables|Default|SetTarget%20Found true))
    (:else
      (Variables|Default|SetTarget%20Found false))))

(event EventBeginPlay
  ;[0.3646 0.3646 0.3646] Call the delete function
  (CallFunction|Delete))

(fn ConstructionScript)

(fn ThrowDirection
  (params (TargetLocked :type Boolean))
  ;[0 1 0.8004] Start
  (bind _actortarget (Variables|Default|GetActorTarget)
    (:then
      ;[1 1 1] Branch
      (if TargetLocked
        ;[0.05725 0 1] Moving Target
        (bind _target_component (Class|Interact|GetTarget(Message) _actortarget))
        (Utilities|IsValid _target_component
          (:Is%20Valid
            (return (* (- (Transformation|GetWorldLocation _target_component) (Transformation|GetActorLocation)) (/ (Variables|Default|GetSpeed) 5e+02))))
          (:Is%20Not%20Valid
            ;[0 1 0.08041] Target
            (return (* (- (Transformation|GetActorLocation _actortarget) (Transformation|GetActorLocation)) (/ (Variables|Default|GetSpeed) 5e+02)))))
        (else
          _)))
    (:else
      _))
  ;[1 0 0] No Target
  (return (* (Transformation|GetActorForwardVector (Game|GetPlayerCharacter 0)) (Variables|Default|GetSpeed))))